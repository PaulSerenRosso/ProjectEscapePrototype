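; Menu game mode that handles online session callbacks for hosting and joining a game.
; When session creation completes it starts the session, and a successful start opens FirstPersonMap as a listen server.
; When a session search completes it retries joining the hardcoded "POMME" session on a short delay loop, with no attempt limit, until the join call returns true.
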(event EventBeginPlay)

(event EventTick
  (params (DeltaSeconds :type Float%20%28single-precision%29)))

(event EventOnCreateSessionComplete
  (params (Name :type Name :default "None") (bArg :type Boolean))
  (Class|MenuGameMode|StartSession (Utilities|String|ToString(Name) Name) bArg))

(event EventOnFindSessionComplete
  (params (bArg :type Boolean))
  (Development|PrintString "try to join Sessions")
  (bind _returnvalue (Class|MenuGameMode|JoinSession "POMME" :!label _label))
  (if _returnvalue
    (Development|PrintString (Utilities|String|Append "State :" (Utilities|String|ToString(Boolean) _returnvalue)))
    (else
      (Utilities|FlowControl|Delay 0.2)
      (goto _label))))

(event EventOnStartSessionComplete
  (params (Name :type Name :default "None") (bArg :type Boolean))
  (if bArg
    (Development|PrintString (Utilities|String|Append "Session \"" (Utilities|String|ToString(Name) Name) "\" was created"))
    (Game|OpenLevel(byName) "FirstPersonMap" true "listen")))

(fn ConstructionScript)